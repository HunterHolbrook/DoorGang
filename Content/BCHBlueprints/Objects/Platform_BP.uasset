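; Platform_BP is an elevator platform that moves once when a character enters its trigger.
; BeginPlay records the platform's starting relative location.
; An overlap by an actor whose display name contains "character" passes a DoOnce, then after a short delay plays elevator music and runs the MovePlatform timeline.
; The timeline lerps the platform's relative location from that start toward PlatformLocationEnd without sweeping.
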(event OnComponentBeginOverlap(PlatformTrigger)
  (params (OverlappedComponent :type Primitive%20Component%20Object%20Reference) (OtherActor :type Actor%20Object%20Reference) (OtherComp :type Primitive%20Component%20Object%20Reference) (OtherBodyIndex :type Integer) (bFromSweep :type Boolean) (SweepResult :type Hit%20Result%20Structure%20%28by%20ref%29))
  ;[1 1 1] Platform Move
  (if (Utilities|String|Contains (Utilities|GetDisplayName OtherActor) "character")
    (Utilities|FlowControl|DoOnce false
      (:Completed
        (Utilities|FlowControl|Delay 0.5)
        (Audio|PlaySound2D "/Game/BCHBlueprints/Audio/ElevatorMusic.ElevatorMusic" 1.0 1.0 0.0 0 0)
        (bind _raiseplatform (Timeline|MovePlatform Play)
          (:Update
            (Transformation|SetRelativeLocation (Variables|Default|GetPlatform) (Math|Vector|Lerp(Vector) (Variables|Default|GetPlatformLocationBegin) (Variables|Default|GetPlatformLocationEnd) _raiseplatform) false false)))))))

(event EventBeginPlay
  ;[1 1 1] Get Begin Location of Platform
  (Variables|Default|SetPlatformLocationBegin (Variables|/Script/Engine.SceneComponent|GetRelativeLocation (Variables|Default|GetPlatform))))

(fn ConstructionScript)