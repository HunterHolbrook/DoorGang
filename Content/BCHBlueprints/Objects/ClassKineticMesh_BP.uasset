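; Tutorial actor in which Thomas rushes to a set spot and plays a voice tutorial when the character enters its trigger volumes.
; MovingCollision plays the ThomasRun timeline, lerping Thomas from his current relative location to a hard-coded target.
; TutorialCollision plays the sound after a short delay at Face's relative location, used as world position.
; Both match "character" in display names, but DoOnce precedes the tutorial's check, so any first overlap consumes it.
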(event OnComponentBeginOverlap(MovingCollision)
  (params (OverlappedComponent :type Primitive%20Component%20Object%20Reference) (OtherActor :type Actor%20Object%20Reference) (OtherComp :type Primitive%20Component%20Object%20Reference) (OtherBodyIndex :type Integer) (bFromSweep :type Boolean) (SweepResult :type Hit%20Result%20Structure%20%28by%20ref%29))
  (bind _thomas (Variables|Default|GetThomas))
  ;[1 1 1] Thomas Moves Toward Player
  (if (Utilities|String|Contains (Utilities|GetDisplayName OtherActor) "character")
    (bind _therushdown (Timeline|ThomasRun Play)
      (:Update
        (Transformation|SetRelativeLocation _thomas (Math|Vector|Lerp(Vector) (Variables|/Script/Engine.SceneComponent|GetRelativeLocation _thomas) "0.000859,725.000000,83.000000" _therushdown) false false)))))

(event OnComponentBeginOverlap(TutorialCollision)
  (params (OverlappedComponent :type Primitive%20Component%20Object%20Reference) (OtherActor :type Actor%20Object%20Reference) (OtherComp :type Primitive%20Component%20Object%20Reference) (OtherBodyIndex :type Integer) (bFromSweep :type Boolean) (SweepResult :type Hit%20Result%20Structure%20%28by%20ref%29))
  ;[1 1 1] Thomas Gives Tutorial
  (Utilities|FlowControl|DoOnce false
    (:Completed
      (if (Utilities|String|Contains (Utilities|GetDisplayName OtherActor) "character")
        (Utilities|FlowControl|Delay 0.5)
        (Audio|PlaySoundatLocation "/Game/BCHBlueprints/Audio/ThomasTutorial.ThomasTutorial" (Variables|/Script/Engine.SceneComponent|GetRelativeLocation (Variables|Default|GetFace)) "0, 0, 0" 1.0 1.0 0.0 0 0 0)))))

(fn ConstructionScript)